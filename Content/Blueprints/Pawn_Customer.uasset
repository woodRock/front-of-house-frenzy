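; Customer pawn that can be teleported to a seat and can pick a random order.
; Its trigger box shows a text render and enables player input on overlap, then reverses both and hides the mouse cursor on exit.
; SeatFunction moves a given customer to the first seat of a four-seat object and sets the isSeated blackboard key.
; GetOrder returns a random entry from AllItems.
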(event OnComponentEndOverlap(Box)
  (params (OverlappedComponent :type Primitive%20Component%20Object%20Reference) (OtherActor :type Actor%20Object%20Reference) (OtherComp :type Primitive%20Component%20Object%20Reference) (OtherBodyIndex :type Integer))
  (bind _returnvalue (Game|GetPlayerController 0))
  (Rendering|SetVisibility (Variables|Default|GetTextRender) false false)
  (Input|DisableInput _returnvalue)
  (Variables|/Script/Engine.PlayerController|SetbShowMouseCursor _returnvalue false))

(event OnComponentBeginOverlap(Box)
  (params (OverlappedComponent :type Primitive%20Component%20Object%20Reference) (OtherActor :type Actor%20Object%20Reference) (OtherComp :type Primitive%20Component%20Object%20Reference) (OtherBodyIndex :type Integer) (bFromSweep :type Boolean) (SweepResult :type Hit%20Result%20Structure%20%28by%20ref%29))
  (Rendering|SetVisibility (Variables|Default|GetTextRender) true false)
  (Input|EnableInput (Game|GetPlayerController 0)))

(fn ConstructionScript)

(fn SeatFunction
  (params (Customer :type Pawn%20Customer%20Object%20Reference) (4seat :type BP%204seater%20Table%20Object%20Reference))
  (Development|PrintString "SeatFunction")
  (Transformation|Teleport Customer (Transformation|GetWorldLocation (Variables|/Game/Blueprints/BP_4seaterTable.BP_4seaterTable_C|GetCustomerSeat1 4seat)) "0, 0, 0")
  (AI|Components|Blackboard|SetValueasBool (AI|GetBlackboard Customer) (Utilities|Name|MakeLiteralName "isSeated") true))

(fn GetOrder
  (bind _allitems (Variables|Default|GetAllItems))
  (return (Utilities|Array|Get(acopy) _allitems (Math|Random|RandomInteger (Utilities|Array|Length _allitems)))))