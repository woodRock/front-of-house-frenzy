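; MyInstance holds shared state for what appears to be a restaurant game: orders, walkouts and coins.
; AddDish appends a random entry from Dishes to Orders, and IncreaseCoins adds a fixed reward to Coins.
; IncreaseWalkouts counts walkouts and, on reaching MaxWalkouts, shows the GameOver widget with the mouse cursor and pauses the game.
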(fn AddDish
  (bind _dishes (Variables|Default|GetDishes))
  (Utilities|Array|Add (Variables|Default|Getorders) (Utilities|Array|Get(acopy) _dishes (Math|Random|RandomInteger (Utilities|Array|Length _dishes)))))

(fn IncreaseWalkouts
  ;[1 1 1] Add a walkout
  (Variables|Default|SetWalkouts (+ (Variables|Default|GetWalkouts) 1))
  ;[1 1 1] Check Lose Condition
  (if (== (Variables|Default|GetWalkouts) (Variables|Default|GetMaxWalkouts))
    ;[1 1 1] Game Over Screen
    (bind _returnvalue (UserInterface|CreateWidget "/Game/Widgets/GameOver.GameOver_C"))
    (UserInterface|Viewport|AddtoViewport _returnvalue 0)
    (Variables|/Script/Engine.PlayerController|SetbShowMouseCursor (Game|GetPlayerController 0) true)
    (Game|SetGamePaused true)))

(fn IncreaseCoins
  (Variables|Default|SetCoins (+ (Variables|Default|GetCoins) 10)))