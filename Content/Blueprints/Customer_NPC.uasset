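; Customer NPC Blueprint with a patience meter that drains over time until the player attends to it.
; Patience starts at its maximum on BeginPlay and drops by a fixed step each Tick while non-negative, so the drain rate depends on frame rate.
; When the player character overlaps ServerTrigger, the current value prints for testing and patience refills to maximum.
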(event OnComponentBeginOverlap(ServerTrigger)
  (params (OverlappedComponent :type Primitive%20Component%20Object%20Reference) (OtherActor :type Actor%20Object%20Reference) (OtherComp :type Primitive%20Component%20Object%20Reference) (OtherBodyIndex :type Integer) (bFromSweep :type Boolean) (SweepResult :type Hit%20Result%20Structure%20%28by%20ref%29))
  ;[1 1 1] Server interaction with customer resets their patience
  ;;[1 1 1] Customer overlapped with the server
  (if (== OtherActor (Game|GetPlayerCharacter 0))
    ;;[1 1 1] Print patience (testing only)
    (Development|PrintString (Utilities|String|ToString(Float) (Variables|Default|GetPatience)))
    ;;[1 1 1] Replenish patience
    (Variables|Default|SetPatience (Variables|Default|GetMaximumPatience))))

(event EventBeginPlay
  ;[1 1 1] Initialize patience at maximuim
  (Variables|Default|SetPatience (Variables|Default|GetMaximumPatience)))

(event EventTick
  (params (DeltaSeconds :type Float%20%28single-precision%29))
  ;[1 1 1] Patience deteriotes each game tick
  ;;[1 1 1] Patience cannot be negative
  (if (>= (Variables|Default|GetPatience) 0.0)
    ;;[1 1 1] Deteriorate Patience
    (Variables|Default|SetPatience (- (Variables|Default|GetPatience) 0.01))))

(event Input|ActionEvents|InputActionLeftClick
  (params (Key :type Key%20Structure :default "None")))

(fn ConstructionScript)