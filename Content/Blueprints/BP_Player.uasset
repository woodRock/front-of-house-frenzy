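; BP_Player is the player-controlled pawn, moved along world X and Y by the LeftRight and UpDown axes.
; Tick smoothly turns the Cube component toward the input direction with a rotation lerp.
; BeginPlay adds the GameUI widget and sets game-only input.
; M shows a cached PauseMenu with cursor and UI-only input, but calls SetGamePaused with false, so the game keeps running.
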(event EventBeginPlay
  ;[1 1 1] Add HUD to character when the game starts
  (bind _returnvalue (UserInterface|CreateWidget "/Game/Widgets/GameUI.GameUI_C"))
  (UserInterface|Viewport|AddtoViewport _returnvalue 0)
  (Input|SetInputModeGameOnly (Game|GetPlayerController 0)))

(event EventTick
  (params (DeltaSeconds :type Float%20%28single-precision%29))
  (if (or (!= (Input|AxisValues|GetUpDown) 0.0) (!= 0.0 (Input|AxisValues|GetLeftRight)))
    ;[1 1 1] set wanted direction
    (Variables|Default|Setdirection (Math|Vector|MakeVector (Input|AxisValues|GetLeftRight) (Input|AxisValues|GetUpDown) 0.0))
    (Transformation|SetWorldRotation (Variables|Default|GetCube) (Math|Rotator|Lerp(Rotator) (Transformation|GetWorldRotation (Variables|Default|GetCube)) (Math|Conversions|RotationFromXVector (Variables|Default|Getdirection)) (* DeltaSeconds (Variables|Default|GetrotationSpeed)) true) false false)))

(event Input|AxisEvents|InputAxisUpDown
  (params (AxisValue :type Float%20%28single-precision%29))
  ;[1 1 1] Movement
  (Pawn|Input|AddMovementInput "0.000000,1.000000, 0" AxisValue false))

(event Input|AxisEvents|InputAxisLeftRight
  (params (AxisValue :type Float%20%28single-precision%29))
  ;[1 1 1] Movement
  (Pawn|Input|AddMovementInput "1.000000,0.000000, 0" AxisValue false))

(event Input|KeyboardEvents|M
  (params (Key :type Key%20Structure :default "None"))
  (bind _returnvalue (Game|GetPlayerController 0))
  ;[1 1 1] Pause the game when the player pushes M
  (:Pressed
    (Utilities|IsValid (Variables|Default|GetPause%20Menu%20Reference)
      (:Is%20Valid
        _)
      (:Is%20Not%20Valid
        (bind _returnvalue_2 (UserInterface|CreateWidget "/Game/Widgets/PauseMenu.PauseMenu_C"))
        (Variables|Default|SetPause%20Menu%20Reference _returnvalue_2)))
    (Variables|/Script/Engine.PlayerController|SetbShowMouseCursor _returnvalue true)
    (Input|SetInputModeUIOnly _returnvalue 0 "DoNotLock")
    (UserInterface|Viewport|AddtoViewport (Variables|Default|GetPause%20Menu%20Reference) 0)
    (Game|SetGamePaused false)))

(fn ConstructionScript)